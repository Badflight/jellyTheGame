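; A 2D Paper melee enemy character that flags a seen player in its AI Blackboard and attacks with a leaping slam.
; LaunchTest turns it toward the player, launches it upward and forward scaled by distance, then issues AIMoveTo on the player.
; Landing runs a debug-drawn sphere trace that damages a hit player, gated by MadeSphere, which is never reset here.
; Incoming damage reduces Health and destroys the actor at zero or below.
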(event OnSeePawn(PawnSensorComp)
  (params (Pawn :type Pawn%20Object%20Reference))
  (Utilities|Casting|CastToBP_ThirdPersonCharacter Pawn)
  (AI|Components|Blackboard|SetValueasBool (AI|GetBlackboard (AI|GetAIController self)) (Utilities|Name|MakeLiteralName "SeenAPlayer") true))

(event Custom|LaunchTest
  (bind _returnvalue (Transformation|GetActorForwardVector))
  (Variables|Default|SetDistance (Transformation|GetDistanceTo (Game|GetPlayerCharacter 0)))
  (Transformation|SetActorRotation (Math|Rotator|MakeRotator 0.0 0.0 (.yaw (Math|Rotator|FindLookatRotation (Transformation|GetActorLocation) (Transformation|GetActorLocation (Game|GetPlayerCharacter 0))))))
  (Character|LaunchCharacter (Math|Vector|MakeVector (* (.x _returnvalue) (Variables|Default|GetDistance)) (* (.y _returnvalue) (Variables|Default|GetDistance)) (+ (.z _returnvalue) 1e+03)) false false)
  (AI|AIMoveTo self "0, 0, 0" (Game|GetPlayerCharacter 0) 5.0 false))

(event EventBeginPlay)

(event Game|Damage|EventAnyDamage
  (params (Damage :type Float%20%28single-precision%29) (DamageType :type Damage%20Type%20Object%20Reference) (InstigatedBy :type Controller%20Object%20Reference) (DamageCauser :type Actor%20Object%20Reference))
  (bind _output_get (Variables|Default|SetHealth (- (Variables|Default|GetHealth) Damage)))
  (Development|PrintString "Damage")
  (if (<= _output_get 0.0)
    (Actor|DestroyActor)))

(event EventOnLanded
  (params (Hit :type Hit%20Result%20Structure%20%28by%20ref%29))
  (bind _returnvalue (Transformation|GetActorLocation))
  (if (Variables|Default|GetMadeSphere)
    (Development|PrintString "Sphere already made")
    (else
      (bind _outhit (Collision|SphereTraceByChannel _returnvalue _returnvalue 9e+01 "TraceTypeQuery1" false 0 "ForDuration"))
      (bind _asbp_third_person_character (Utilities|Casting|CastToBP_ThirdPersonCharacter (.HitActor (Collision|BreakHitResult _outhit)))
        (:then
          (Development|PrintString "Hit player")
          (Game|Damage|ApplyDamage _asbp_third_person_character (Variables|Default|GetBase%20Damage) 0 0))
        (:CastFailed
          (Development|PrintString "Did not hit player")))
      (Variables|Default|SetMadeSphere true))))

(fn ConstructionScript)