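; Salt King AI helper that spawns spikes at five fixed scene-component points, leaving one chosen point safe.
; SpawnSafeCube only rolls and stores the safe index; it spawns no cube.
; SpawnSpike spawns SpikeOnPlayerBP at every point except that index, with debug prints.
; The inclusive random range reaches the array length, so a roll can leave no safe point.
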(event Custom|SpawnSpike
  (Development|PrintString (Utilities|String|ToString(Integer) (Variables|Default|GetRandomInteger)))
  (for (_array_element _array_index) (Variables|Default|GetSceneCompRef)
    (if (== _array_index (Variables|Default|GetRandomInteger))
      (Development|PrintString (Utilities|String|ToString(Integer) (Variables|Default|GetRandomInteger)))
      (else
        (Game|SpawnActorfromClass "/Game/AI/SaltKing/SpikeOnPlayerBP.SpikeOnPlayerBP_C" (Math|Transform|MakeTransform (.location (Transformation|GetWorldTransform _array_element)) "0, 0, 0" "1.000000,1.000000,1.000000") "Undefined" 0 0)))))

(event Custom|SpawnSafeCube
  (Variables|Default|SetRandomInteger (Math|Random|RandomIntegerinRange 0 (Utilities|Array|Length (Variables|Default|GetSceneCompRef))))
  (Development|PrintString "Spawn Safe Cube"))

(event EventBeginPlay
  (Variables|Default|SetSceneCompRef (Utilities|Array|MakeArray (Variables|Default|GetScene) (Variables|Default|GetScene1) (Variables|Default|GetScene2) (Variables|Default|GetScene3) (Variables|Default|GetScene4))))

(fn ConstructionScript)