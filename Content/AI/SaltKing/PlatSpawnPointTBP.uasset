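; PlatSpawnPointTBP is a Salt King spawn-point Blueprint that creates temporary platforms at a fixed set of locations.
; BeginPlay gathers five scene components into an array to serve as markers.
; The SpawnPlatform event spawns a TempPlatFormBP at each marker's world location with zero rotation, printing a debug string per spawn.
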(event Custom|SpawnPlatform
  (for _array_element (Variables|Default|GetArrayOfSceneComp)
    (Game|SpawnActorfromClass "/Game/AI/SaltKing/TempPlatFormBP.TempPlatFormBP_C" (Math|Transform|MakeTransform (.location (Transformation|GetWorldTransform _array_element)) "0,0.000000, 0" "1.000000,1.000000,1.000000") "Undefined" 0 0)
    (Development|PrintString "Hello")))

(event EventBeginPlay
  (Variables|Default|SetArrayOfSceneComp (Utilities|Array|MakeArray (Variables|Default|GetScene) (Variables|Default|GetScene1) (Variables|Default|GetScene2) (Variables|Default|GetScene3) (Variables|Default|GetScene4))))

(fn ConstructionScript)